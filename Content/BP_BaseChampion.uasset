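; BP_BaseChampion is a base champion unit that shows an overhead health bar with the champion's name.
; On BeginPlay it casts its widget component's widget to unit_HealthBar, makes it visible, and seeds health values and the name from ChosenChampion.
; Each Tick it pushes current and base health into the widget, repositions the component above the capsule and disables its shadow casting.
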(event EventBeginPlay
  (bind _healthbarwidgetcomponent (Variables|Default|GethealthBarWidgetComponent))
  (bind _returnvalue (UserInterface|GetUserWidgetObject _healthbarwidgetcomponent))
  (bind _asunit_health_bar (Utilities|Casting|CastTounit_HealthBar _returnvalue))
  (Widget|SetVisibility _returnvalue "Visible")
  (Widget|SetVisibility _asunit_health_bar "Visible")
  (Class|WidgetComponent|SetTickwhenOffscreen (Variables|Default|GethealthBarWidgetComponent) true)
  (Variables|/Game/Widgets/unit_HealthBar.unit_HealthBar_C|SetHealthPercent _asunit_health_bar (Variables|Default|GetcurrentHealth))
  (Variables|/Game/Widgets/unit_HealthBar.unit_HealthBar_C|SetMaxHealth _asunit_health_bar (Variables|Default|GetbaseHealth))
  (Variables|/Game/Widgets/unit_HealthBar.unit_HealthBar_C|SetChampName _asunit_health_bar (Utilities|Text|ToText(String) (Variables|Default|GetchosenChampion))))

(event Collision|EventActorBeginOverlap
  (params (OtherActor :type Actor%20Object%20Reference)))

(event EventTick
  (params (DeltaSeconds :type Float%20%28single-precision%29))
  (Variables|/Game/Widgets/unit_HealthBar.unit_HealthBar_C|SetHealthPercent (stale EventBeginPlay _asunit_health_bar) (Variables|Default|GetcurrentHealth))
  (Variables|/Game/Widgets/unit_HealthBar.unit_HealthBar_C|SetMaxHealth (stale EventBeginPlay _asunit_health_bar) (Variables|Default|GetbaseHealth))
  (Transformation|SetWorldLocation (Variables|Default|GethealthBarWidgetComponent) (+ (Transformation|GetWorldLocation (Variables|Default|GetCapsuleComponent)) "-15.000000,0.000000,150.000000") false false)
  (Rendering|SetCastShadow (Variables|Default|GethealthBarWidgetComponent) false))

(fn ConstructionScript)